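; Blueprint function library of shared gameplay helpers for player damage, pickups, scoring, ammo and actor toggling.
; TakeDamage reduces Shield while Shield+HP stays above 100, otherwise zeroes it and cuts HP, triggering low-HP or death events.
; Shield and health helpers clamp values and update the HUD, while AddPoints feeds Score and Money with optional doubling.
; ManageAmmo reads or writes per-gun ammo in BP_GameInstance; SaveData is empty and the damage sound is disconnected.
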(fn `ActivateObject`
  (params (Actor :type "Actor Object Reference") (Disabled :type Boolean))
  (bind _returnvalue (not Disabled))
  ;[1 1 1] Activate or Deactivate an Actor
  (`Actor.SetActorHiddenInGame` Actor Disabled)
  (`Actor.SetActorEnableCollision` Actor _returnvalue)
  (`Actor.SetActorTickEnabled` Actor _returnvalue)
  (return))

(fn `AddHealth`
  (params (`BP Player` :type "/Game/Blueprints/Player/BP_Player Object Reference") (`Amount of Health` :type Integer))
  (bind _returnvalue (`KismetMathLibrary.Clamp` (+ (`/Game/Blueprints/Player/BP_Player.HP` `BP Player`) `Amount of Health`) 0 100))
  ;[1 1 1] Add Health
  (set `/Game/Blueprints/Player/BP_Player.HP` _returnvalue `BP Player`)
  ;[1 1 1] If Player had Low HP and obtains HP, eliminate Blood Effect
  (if (> _returnvalue 10)
    (`/Game/Blueprints/Interface/HUDS/WBP_HUD.CE_GoodHP` (`/Game/Blueprints/Player/BP_Player.HUD` `BP Player`))))

(fn `AddPoints`
  (params (Points :type Integer) (Object :type "/Game/Blueprints/Player/BP_Player Object Reference"))
  (locals (PointsToAdd :type Integer))
  ;[1 1 1] Add Points To Score And Money
  (if (`/Game/Blueprints/Player/BP_Player.IsX2Activated` Object)
    (set `local.PointsToAdd` (* Points 2))
    (else
      (set `local.PointsToAdd` Points)))
  (set `/Game/Blueprints/Player/BP_Player.Score` (+ (`/Game/Blueprints/Player/BP_Player.Score` Object) (`local.PointsToAdd`)) Object)
  (set `/Game/Blueprints/Player/BP_Player.Money` (+ (`/Game/Blueprints/Player/BP_Player.Money` Object) (`local.PointsToAdd`)) Object))

(fn `AddShield`
  (params (`BP Player` :type "/Game/Blueprints/Player/BP_Player Object Reference") (AmountOfShield :type Integer))
  ;[1 1 1] Add Shield
  (set `/Game/Blueprints/Player/BP_Player.Shield` (`KismetMathLibrary.Clamp` (+ (`/Game/Blueprints/Player/BP_Player.Shield` `BP Player`) AmountOfShield) 0 100) `BP Player`)
  ;[1 1 1] Change Image to Shield
  (`Image.SetBrushFromTexture` (`/Game/Blueprints/Interface/HUDS/WBP_HUD.I_HeartShield` (`/Game/Blueprints/Player/BP_Player.HUD` `BP Player`)) "/Game/Texturas/User_Interface/SHieldUI.SHieldUI" false))

(fn `ManageAmmo`
  (params (Gun :type "/Game/Blueprints/Enums/Enum_Weapons Enum" :default "NewEnumerator3") (IsGettingAmmo :type Boolean) (NewAmmo :type Integer) (NewCurrentLoad :type Integer))
  (returns (Ammo :type Integer) (CurrentLoad :type Integer))
  (locals (GameInstance :type "/Game/Blueprints/BP_GameInstance Object Reference"))
  (bind _gameinstance (`local.GameInstance`))
  (bind _gameinstance_2 (`local.GameInstance`))
  (bind _gameinstance_3 (`local.GameInstance`))
  (bind _gameinstance_4 (`local.GameInstance`))
  (bind _asbp_game_instance (cast `/Game/Blueprints/BP_GameInstance` (`GameplayStatics.GetGameInstance` null)))
  (set `local.GameInstance` _asbp_game_instance)
  (switch `/Game/Blueprints/Enums/Enum_Weapons` Gun
    (:`NewEnumerator1`
      (if IsGettingAmmo
        (return (`/Game/Blueprints/BP_GameInstance.AmmoPistol` _gameinstance) (`/Game/Blueprints/BP_GameInstance.CurrentLoadPistol` _gameinstance))
        (else
          (set `/Game/Blueprints/BP_GameInstance.AmmoPistol` NewAmmo (`local.GameInstance`))
          (set `/Game/Blueprints/BP_GameInstance.CurrentLoadPistol` NewCurrentLoad (`local.GameInstance`)))))
    (:`NewEnumerator2`
      (if IsGettingAmmo
        (return (`/Game/Blueprints/BP_GameInstance.AmmoRifle` _gameinstance_3) (`/Game/Blueprints/BP_GameInstance.CurrentLoadRifle` _gameinstance_3))
        (else
          (set `/Game/Blueprints/BP_GameInstance.AmmoRifle` NewAmmo (`local.GameInstance`))
          (set `/Game/Blueprints/BP_GameInstance.CurrentLoadRifle` NewCurrentLoad (`local.GameInstance`)))))
    (:`NewEnumerator4`
      (if IsGettingAmmo
        (return (`/Game/Blueprints/BP_GameInstance.AmmoShotgun` _gameinstance_4) (`/Game/Blueprints/BP_GameInstance.CurrentLoadShotgun` _gameinstance_4))
        (else
          (set `/Game/Blueprints/BP_GameInstance.AmmoShotgun` NewAmmo (`local.GameInstance`))
          (set `/Game/Blueprints/BP_GameInstance.CurrentLoadShotgun` NewCurrentLoad (`local.GameInstance`)))))
    (:`NewEnumerator5`
      (if IsGettingAmmo
        (return (`/Game/Blueprints/BP_GameInstance.AmmoSniper` _gameinstance_2) (`/Game/Blueprints/BP_GameInstance.CurrentLoadSniper` _gameinstance_2))
        (else
          (set `/Game/Blueprints/BP_GameInstance.AmmoSniper` NewAmmo (`local.GameInstance`))
          (set `/Game/Blueprints/BP_GameInstance.CurrentLoadSniper` NewCurrentLoad (`local.GameInstance`)))))))

(fn `SaveData`
  (locals (HP :type Integer) (Score :type Integer)))

(fn `TakeDamage`
  (params (Object :type "Actor Object Reference") (Damage :type Integer))
  (locals (`Shield-Damage` :type Integer) (`HP-Damage` :type Integer) (AsBPPlayer :type "/Game/Blueprints/Player/BP_Player Object Reference"))
  (bind _asbpplayer (`local.AsBPPlayer`))
  (bind _asbp_player (cast `/Game/Blueprints/Player/BP_Player` Object))
  (bind _output_get (set `local.AsBPPlayer` _asbp_player))
  (`/Game/Blueprints/Player/BP_Player.CE_HitAnimation` _output_get)
  (bind _shield (`/Game/Blueprints/Player/BP_Player.Shield` _asbp_player))
  (set `local.Shield-Damage` (- _shield (`local.Damage`)))
  (bind _hp (`/Game/Blueprints/Player/BP_Player.HP` _asbp_player))
  (set `local.HP-Damage` (- _hp Damage))
  (if (> (- (+ _shield _hp) (`local.Damage`)) 100)
    ;[1 1 1] Damage Only Affects Shield
    (set `/Game/Blueprints/Player/BP_Player.Shield` (`local.Shield-Damage`) (`local.AsBPPlayer`))
    (else
      ;[1 1 1] Damage Affects HP and Can Affect Shield
      (set `/Game/Blueprints/Player/BP_Player.HP` (`local.HP-Damage`) _asbpplayer)
      (set `/Game/Blueprints/Player/BP_Player.Shield` 0 _asbpplayer)
      ;[1 1 1] Change Image to Heart
      (`Image.SetBrushFromTexture` (`/Game/Blueprints/Interface/HUDS/WBP_HUD.I_HeartShield` (`/Game/Blueprints/Player/BP_Player.HUD` _asbpplayer)) "/Game/Texturas/User_Interface/Heart_container.Heart_container" false)
      ;[1 1 1] Check if Player is Dead
      (if (== 0 (`/Game/Blueprints/Player/BP_Player.HP` _asbpplayer))
        (`/Game/Blueprints/Player/BP_Player.CE_Die` _asbpplayer)
        (else
          ;[1 1 1] Check if Low HP
          (if (<= (`/Game/Blueprints/Player/BP_Player.HP` _asbpplayer) 10)
            (`/Game/Blueprints/Interface/HUDS/WBP_HUD.CE_LowHP` (`/Game/Blueprints/Player/BP_Player.HUD` _asbpplayer))))))))