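; Interactive checkpoint that, once triggered, records itself in the game instance and starts the next round.
; Interaction passes a DoOnce gate, plays a sound, turns the mesh yellow and resets any previous, different checkpoint.
; A timeline then shrinks the mesh alongside particles, disables the actor, restores its scale, fires the disappearance dispatcher and calls the game mode.
; Resetting restores the material and re-arms the gate.
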(event `self.CE_Interact`
  ;[1 1 1] CheckPoint
  (`/Engine/EditorBlueprintResources/StandardMacros.DoOnce` false :!label _label
    (:`Completed`
      (`GameplayStatics.PlaySound2D` "/Game/Audio/Cues/C_Checkpoint_Cue.C_Checkpoint_Cue" 1.0 1.0 0.0 null null)
      (`PrimitiveComponent.SetMaterial` (`self.Mesh`) 0 "/Game/Materials/M_Translucent_Yellow.M_Translucent_Yellow")
      (bind _asbp_game_instance (cast `/Game/Blueprints/BP_GameInstance` (`GameplayStatics.GetGameInstance`)))
      (bind _output (`|ConvertAsset` (`/Game/Blueprints/BP_GameInstance.LastCheckpoint` _asbp_game_instance)))
      (`/Engine/EditorBlueprintResources/StandardMacros.IsValid` _output
        (:`Is Valid`
          (if (!= self _output)
            (`self.CE_Reset` _output)
            (set `/Game/Blueprints/BP_GameInstance.LastCheckpoint` (`|ConvertAsset` self) _asbp_game_instance :!label _label_2)
            ;;[1 1 1] Particles
            (`ActorComponent.Activate` (`self.P_CheckpointParticles_System`) false)
            ;;[1 1 1] Shrinks and Disappears
            (set `self.StartScale` (`SceneComponent.RelativeScale3D` (`self.Mesh`)))
            (bind (_direction _scale) (`Timeline|TM_Shrink`)
              (:`Update`
                (`SceneComponent.SetRelativeScale3D` (`self.Mesh`) (`KismetMathLibrary.VLerp` (0.0 0.0 0.0) (`self.StartScale`) _scale)))
              (:`Finished`
                (`/Game/Blueprints/BP_FunctionLibrary.ActivateObject` self true)
                (`SceneComponent.SetRelativeScale3D` (`self.Mesh`) (`self.StartScale`))
                (`self.CheckPointDissapears`)
                ;;[1 1 1] When Checkpoint is activated, start next round
                (bind _asbp_base_game_mode (cast `/Game/Blueprints/GameModes/BP_BaseGameMode` (`GameplayStatics.GetGameMode`)))
                (`/Game/Blueprints/GameModes/BP_BaseGameMode.CE_StartRound` _asbp_base_game_mode)))))
        (:`Is Not Valid`
          (goto _label_2))))))

(event `CE_Reset`
  ;[1 1 1] CheckPoint
  (`PrimitiveComponent.SetMaterial` (`self.Mesh`) 0 "/Game/Materials/M_Translucent.M_Translucent")
  (goto _label :!via `Reset`))

(fn `UserConstructionScript`
  (`parent.UserConstructionScript`))