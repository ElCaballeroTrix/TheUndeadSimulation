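; Base interactive object that reacts when the player overlaps it, with an empty interact event as the hook for specific behavior.
; If it needs input, overlap enables input and shows a HUD prompt with a click sound, and the Interact action fires the event; otherwise overlap fires it immediately.
; Leaving disables input and hides the prompt.
; BeginPlay adds the general input mapping and caches the player's HUD for input-driven objects.
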(event `self.ReceiveBeginPlay`
  ;[0.2001 1 0] BeginPlay
  (if (`self.NeedsInput`)
    (`EnhancedInputSubsystemInterface.AddMappingContext` (pcsubsystem `EnhancedInputLocalPlayerSubsystem` (`GameplayStatics.GetPlayerController` 0)) "/Game/ThirdPerson/Input/IMC_General.IMC_General" 0 (struct))
    (`KismetSystemLibrary.Delay` 0.1)
    (bind _asbp_player (cast `/Game/Blueprints/Player/BP_Player` (`GameplayStatics.GetPlayerPawn` 0)))
    (bind _output_get (set `self.As BP Player` _asbp_player))
    (set `self.HUD` (`/Game/Blueprints/Player/BP_Player.HUD` _output_get))))

(event `self.ReceiveActorBeginOverlap`
  (params (OtherActor :type "Actor Object Reference"))
  ;[1 1 1] Overlaps
  (bind _asbp_player (cast `/Game/Blueprints/Player/BP_Player` OtherActor))
  (`self.Show Interactive Object Text` true (`/Game/Blueprints/Player/BP_Player.HUD` _asbp_player)))

(event `self.ReceiveActorEndOverlap`
  (params (OtherActor :type "Actor Object Reference"))
  ;[1 1 1] Overlaps
  (bind _asbp_player (cast `/Game/Blueprints/Player/BP_Player` OtherActor))
  (`self.Show Interactive Object Text` false (`/Game/Blueprints/Player/BP_Player.HUD` _asbp_player)))

(event `CE_Interact`)

(event `EnhancedInput|/Game/ThirdPerson/Input/Actions/IA_Interact`
  (params (ActionValue :type Boolean) (ElapsedSeconds :type "Float (double-precision)") (TriggeredSeconds :type "Float (double-precision)") (InputAction :type "InputAction Object Reference" :default "/Game/ThirdPerson/Input/Actions/IA_Interact.IA_Interact"))
  ;[1 1 1] Check if it needs Input
  (:`Started`
    (if (`self.NeedsInput`)
      (`self.CE_Interact`))))

(fn `Show Interactive Object Text`
  (params (IsOverlapping :type Boolean) (HUD :type "/Game/Blueprints/Interface/HUDS/WBP_HUD Object Reference"))
  (if IsOverlapping
    ;[1 1 1] Show Text if Needs Input
    (if (`self.NeedsInput`)
      (`self.EnableInput` (`GameplayStatics.GetPlayerController` 0))
      (`/Game/Blueprints/Interface/HUDS/WBP_HUD.CE_MessageText` HUD (`self.Input Text`) "Visible" "/Game/Audio/Waves/S_Click.S_Click")
      (else
        (`self.CE_Interact`)))
    (else
      ;[1 1 1] Hide Text
      (`self.DisableInput` (`GameplayStatics.GetPlayerController` 0))
      (`/Game/Blueprints/Interface/HUDS/WBP_HUD.CE_MessageText` HUD "\"\"" "Hidden" null))))

(fn `UserConstructionScript`)