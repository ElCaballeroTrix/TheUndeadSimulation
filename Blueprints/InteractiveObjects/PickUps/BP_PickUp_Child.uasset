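; Pickup child Blueprint that extends a parent interactive object with idle animation, pickup sound and optional self-destruction.
; A Timeline drives the mesh's vertical bob and rotation, and is stopped on BeginPlay for objects flagged as not animated, such as weapons.
; One destroy flag both starts a timed despawn on BeginPlay and destroys the actor on interaction.
; Interaction plays a sound at the actor's location.
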(event `self.ReceiveBeginPlay`
  ;[0.1419 1 0] Begin Play
  (`parent.ReceiveBeginPlay`)
  (if (`self.ShowBeDestroyedAfterPickUp`)
    (`self.CE_DestroyAfterSomeTime`))
  ;;[0.1266 1 0] Check to see if the interactive object is a weapon, so it won't do the animation
  (if (`self.IsNotAnimated`)
    (bind (_direction _verticalmovement _rotation) (`Timeline|Timeline` :!via `Stop`)
      (:`Update`
        (`SceneComponent.K2_SetRelativeLocationAndRotation` (`self.Mesh`) (`KismetMathLibrary.MakeVector` 0.0 0.0 _verticalmovement) (`KismetMathLibrary.MakeRotator` (`self.RotationX`) 0.0 _rotation) false false)))))

(event `self.CE_Interact`
  (if (`self.ShowBeDestroyedAfterPickUp`)
    (`self.K2_DestroyActor`))
  (`GameplayStatics.PlaySoundAtLocation` (`self.Sound`) (`self.K2_GetActorLocation`) (struct) 1.0 1.0 0.0 null null null null))

(event `CE_DestroyAfterSomeTime`
  (`KismetSystemLibrary.Delay` 20.0)
  (`self.K2_DestroyActor`))

(fn `UserConstructionScript`
  (`parent.UserConstructionScript`))