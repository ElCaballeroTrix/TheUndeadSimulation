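; Respawnable pistol ammo pickup, a child Blueprint that refills the player's pistol ammo when obtained.
; Its obtain-item override sets the pistol ammo stored in BP_GameInstance to its maximum.
; It triggers a reload on BP_Player if the active weapon matches a specific enum entry, presumably the pistol.
; It then hands off to the parent's obtain logic, which is skipped if either cast fails.
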(event `self.CE_ObtainItem`
  (bind _asbp_player (cast `/Game/Blueprints/Player/BP_Player` (`GameplayStatics.GetPlayerPawn` 0)))
  (bind _asbp_game_instance (cast `/Game/Blueprints/BP_GameInstance` (`GameplayStatics.GetGameInstance`)))
  (set `/Game/Blueprints/BP_GameInstance.AmmoPistol` (`/Game/Blueprints/BP_GameInstance.MaxAmmoPistol` _asbp_game_instance) _asbp_game_instance)
  (if (`|EnumEquality` (`/Game/Blueprints/Player/BP_Player.ActiveWeapon` _asbp_player) "NewEnumerator1")
    (`/Game/Blueprints/Player/BP_Player.CE_ReloadWeapon` _asbp_player))
  (`parent.CE_ObtainItem`))

(fn `UserConstructionScript`
  (`parent.UserConstructionScript`))