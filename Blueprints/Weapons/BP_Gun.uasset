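; BP_Gun is a gun actor that fires projectiles and tracks ammo by gun name through ManageAmmo.
; Shooting plays the fire animation, reports noise, traces from the camera and spawns a bullet at the muzzle rotated toward the crosshair target.
; Shotguns add four pellets using shuffled spread rotations, and spawned projectiles receive the player HUD.
; Each shot consumes one round, while Reload refills the magazine from reserve ammo.
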(event `self.ReceiveBeginPlay`
  ;[0.1389 1 0] Begin Play
  ;;[1 1 1] Set Ammo
  (bind (_ammo _currentload) (`/Game/Blueprints/BP_FunctionLibrary.ManageAmmo` (`self.NameOfGun`) true))
  (set `self.Ammo` _ammo)
  (set `self.CurrentLoad` _currentload)
  (`parent.ReceiveBeginPlay`))

(event `CE_Shoot`
  (bind _returnvalue (`GameplayStatics.GetPlayerCameraManager` 0))
  (bind _returnvalue_2 (`SceneComponent.GetSocketLocation` (`self.GunMesh`) "MuzzleFlash"))
  (bind _returnvalue_3 (`self.K2_GetActorLocation` _returnvalue))
  (`SkeletalMeshComponent.PlayAnimation` (`self.GunMesh`) (`self.FireAnimation`) false)
  (`AISense_Hearing.ReportNoiseEvent` (`self.K2_GetActorLocation`) 1.0 (`self.GetParentActor`) 30000.0 "Noise")
  ;[1 1 1] Combine two line traces to spawn a projectile that starts in the gun and ends where the crosshair is aiming
  (bind _outhit (`KismetSystemLibrary.LineTraceSingle` _returnvalue_3 (+ _returnvalue_3 (* (`self.GetActorForwardVector` _returnvalue) 20000)) "TraceTypeQuery1"))
  (bind (_bblockinghit _binitialoverlap _time _distance _location _impactpoint _normal _impactnormal _physmat _hitactor _hitcomponent _hitbonename _bonename _hititem _elementindex _faceindex _tracestart _traceend) (`GameplayStatics.BreakHitResult` _outhit))
  (bind _returnvalue_4 (select `bool` (== _impactpoint (0.0 0.0 0.0)) :`false` _impactpoint :`true` _traceend))
  (`KismetSystemLibrary.LineTraceSingle` :`Start` _returnvalue_2 :`End` _returnvalue_4 :`TraceChannel` "TraceTypeQuery1" :`TraceColor` (struct :`G` 0.196409 :`B` 1.0 :`A` 1.0))
  (bind _returnvalue_5 (`KismetMathLibrary.FindLookAtRotation` _returnvalue_2 _returnvalue_4))
  (`self.CE_SpawnBullet` _returnvalue_2 _returnvalue_5)
  (`self.UseAmmo`)
  ;;[1 0.7553 0] Spawn 5 Bullets for ShotGun
  (if (`self.IsShotgun`)
    (`KismetArrayLibrary.Array_Shuffle` (`self.RandomBulletDirections`))
    (`self.CE_SpawnBullet` _returnvalue_2 (`KismetMathLibrary.ComposeRotators` _returnvalue_5 (`|GetArrayItem` (`self.RandomBulletDirections`))))
    (`self.CE_SpawnBullet` _returnvalue_2 (`KismetMathLibrary.ComposeRotators` _returnvalue_5 (`|GetArrayItem` (`self.RandomBulletDirections`) 1)))
    (`self.CE_SpawnBullet` _returnvalue_2 (`KismetMathLibrary.ComposeRotators` _returnvalue_5 (`|GetArrayItem` (`self.RandomBulletDirections`) 2)))
    (`self.CE_SpawnBullet` _returnvalue_2 (`KismetMathLibrary.ComposeRotators` _returnvalue_5 (`|GetArrayItem` (`self.RandomBulletDirections`) 3)))))

(event `CE_StopShooting`)

(event `CE_SpawnBullet`
  (params (Location :type "Vector Structure") (Rotation :type "Rotator Structure"))
  ;[0 0.02998 1] Spawn Bullet
  (bind _returnvalue (`|SpawnActorFromClass` (`self.Bullet`) (`KismetMathLibrary.MakeTransform` Location Rotation) "AdjustIfPossibleButAlwaysSpawn" "MultiplyWithRoot" self (`GameplayStatics.GetPlayerPawn` 0)))
  (bind _asbp_projectiles (cast `/Game/Blueprints/Weapons/BP_Projectiles` _returnvalue))
  (set `/Game/Blueprints/Weapons/BP_Projectiles.PlayerHUD` (`self.PlayerHUD`) _asbp_projectiles))

(fn `Reload`
  (locals (TempAmmo :type Integer :default 0))
  (bind _ammo (`self.Ammo`))
  ;[1 1 1] Get Ammo of Gun
  (bind (_ammo_2 _currentload) (`/Game/Blueprints/BP_FunctionLibrary.ManageAmmo` (`self.NameOfGun`) true))
  (set `self.Ammo` _ammo_2)
  (set `self.CurrentLoad` _currentload)
  (set `local.TempAmmo` _ammo)
  (set `self.Ammo` (`KismetMathLibrary.Clamp` (- _ammo (- (`self.MaxLoad`) (`self.CurrentLoad`))) 0 (`self.Ammo`)))
  (set `self.CurrentLoad` (+ (- (`local.TempAmmo`) (`self.Ammo`)) (`self.CurrentLoad`)))
  ;[1 1 1] Manage Ammo of Gun
  (`/Game/Blueprints/BP_FunctionLibrary.ManageAmmo` (`self.NameOfGun`) false (`self.Ammo`) (`self.CurrentLoad`)))

(fn `UseAmmo`
  ;[1 1 1] Get Ammo of Gun
  (bind (_ammo _currentload) (`/Game/Blueprints/BP_FunctionLibrary.ManageAmmo` (`self.NameOfGun`) true))
  (set `self.Ammo` _ammo)
  (set `self.CurrentLoad` _currentload)
  (set `self.CurrentLoad` (`KismetMathLibrary.Clamp` (- (`self.CurrentLoad`) 1) 0 (`self.MaxLoad`)))
  (`/Game/Blueprints/BP_FunctionLibrary.ManageAmmo` (`self.NameOfGun`) false (`self.Ammo`) (`self.CurrentLoad`)))

(fn `UserConstructionScript`)