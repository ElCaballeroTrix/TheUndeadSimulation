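; BP_MeleeWeapon is a melee weapon actor that damages zombies its capsule overlaps.
; It disables actor collision on BeginPlay, and this file never re-enables it.
; On capsule overlap it casts to BP_Zombies, then BP_MegaZombie, and calls that class's damage function with its Damage value and no bone or impact point.
; Zombie hits play a knife body impact sound, while anything else plays a surface impact sound.
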(event `self.ReceiveBeginPlay`
  (`self.SetActorEnableCollision` false))

(event `self.Capsule.OnComponentBeginOverlap`
  (params (OverlappedComponent :type "PrimitiveComponent Object Reference") (OtherActor :type "Actor Object Reference") (OtherComp :type "PrimitiveComponent Object Reference") (OtherBodyIndex :type Integer) (bFromSweep :type Boolean) (SweepResult :type "HitResult Structure (by ref)"))
  ;[1 1 1] Damage
  (bind _asbp_zombies (cast `/Game/Blueprints/Zombies/BP_Zombies` OtherActor)
    (:`then`
      (`GameplayStatics.PlaySoundAtLocation` "/Game/MilitaryWeapSilver/Sound/Knife/Cues/Knife_ImpactBody_Cue.Knife_ImpactBody_Cue" (`self.K2_GetActorLocation`) (struct) 1.0 1.0 0.0 null null null null)
      (`/Game/Blueprints/Zombies/BP_Zombies.DamageZombie` _asbp_zombies (`self.Damage`) "None" (0.0 0.0 0.0)))
    (:`CastFailed`
      (bind _asbp_mega_zombie (cast `/Game/Blueprints/Zombies/BP_MegaZombie` OtherActor)
        (:`then`
          (`GameplayStatics.PlaySoundAtLocation` "/Game/MilitaryWeapSilver/Sound/Knife/Cues/Knife_ImpactBody_Cue.Knife_ImpactBody_Cue" (`self.K2_GetActorLocation`) (struct) 1.0 1.0 0.0 null null null null)
          (`/Game/Blueprints/Zombies/BP_MegaZombie.DamageMegaZombie` _asbp_mega_zombie (`self.Damage`) "None" (0.0 0.0 0.0)))
        (:`CastFailed`
          (`GameplayStatics.PlaySoundAtLocation` "/Game/MilitaryWeapSilver/Sound/Knife/Cues/Knife_ImpactSurface_Cue.Knife_ImpactSurface_Cue" (`self.K2_GetActorLocation`) (struct) 1.0 1.0 0.0 null null null null))))))

(fn `UserConstructionScript`)