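; BP_Rifle is a child weapon Blueprint that adds automatic fire to the inherited shooting behavior.
; On BeginPlay it caches its parent actor as BP_Player.
; CEShoot fires through the parent event and opens a Gate, then calls itself after each FireRate delay while the gate is open.
; The loop ends when CEStopShooting closes the gate, or when the player is reloading or the current gun is empty.
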(event `self.ReceiveBeginPlay`
  ;[0.3381 1 0] Begin Play
  (bind _asbp_player (cast `/Game/Blueprints/Player/BP_Player` (`self.GetParentActor`)))
  (set `self.As BP Player` _asbp_player)
  (`parent.ReceiveBeginPlay`))

(event `self.CE_Shoot`
  (bind _as_bp_player (`self.As BP Player`))
  ;[1 1 1] Automatic Shooting
  (`|ExecutionSequence`
    (:`then_0`
      (`parent.CE_Shoot`)
      (`KismetSystemLibrary.Delay` (`self.Fire Rate`))
      (`/Engine/EditorBlueprintResources/StandardMacros.Gate` true :!label _label
        (:`Exit`
          (if (and (not (`/Game/Blueprints/Player/BP_Player.Reloading` _as_bp_player)) (!= (`/Game/Blueprints/Weapons/BP_Gun.CurrentLoad` (`/Game/Blueprints/Player/BP_Player.CurrentGun` _as_bp_player)) 0))
            (`self.CE_Shoot`)
            (else
              (goto _label :!via `Close`))))))
    (:`then_1`
      (goto _label :!via `Open`))))

(event `self.CE_StopShooting`
  ;[1 1 1] Automatic Shooting
  (goto _label :!via `Close`))

(fn `UserConstructionScript`
  (`parent.UserConstructionScript`))