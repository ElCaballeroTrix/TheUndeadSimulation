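; AI controller for BP_Zombies that picks waypoint patrol or behavior tree control at BeginPlay.
; Waypoint zombies disable tick and, after each move completes, pause briefly then claim the first unoccupied BP_Waypoint, clearing occupied flags passed during the search.
; Other zombies run BT_ZombieTree, with tick explicitly enabled because of object pooling, and update the IsAttacking blackboard key from distance to the player.
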(event `self.ReceiveBeginPlay`
  (bind _asbp_zombies (cast `/Game/Blueprints/Zombies/BP_Zombies` (`self.GetInstigator`)))
  (if (`/Game/Blueprints/Zombies/BP_Zombies.FollowsWaypoint` _asbp_zombies)
    ;[1 1 1] Go from a waypoint to the other
    (`self.SetActorTickEnabled` false)
    (add `self.ReceiveMoveCompleted` (delegate `CE_MoveCompleted`))
    (bind _outactors (`GameplayStatics.GetAllActorsOfClass` "/Game/Blueprints/Zombies/BP_Waypoint.BP_Waypoint_C" :!label _label))
    (`KismetSystemLibrary.Delay` 2.0)
    (for _array_element _outactors
      (if (`/Game/Blueprints/Zombies/BP_Waypoint.Occupied` _array_element)
        (set `/Game/Blueprints/Zombies/BP_Waypoint.Occupied` false _array_element)
        (else
          (set `/Game/Blueprints/Zombies/BP_Waypoint.Occupied` true _array_element)
          (`self.MoveToActor` _array_element -1.0 true true true null)
          (break))))
    (else
      (`self.RunBehaviorTree` "/Game/Blueprints/Zombies/AI/BT_ZombieTree.BT_ZombieTree")
      ;[1 1 1] It activates do to Object Pooling. When a zombie dies, its not destroyed, its inactive
      (`self.SetActorTickEnabled` true))))

(event `CE_MoveCompleted` :!signature `self.ReceiveMoveCompleted`
  (params (RequestID :type "AIRequestID Structure") (Result :type "EPathFollowingResult Enum" :default "Success"))
  ;[1 1 1] Go from a waypoint to the other
  (goto _label))

(event `self.ReceiveTick`
  (params (DeltaSeconds :type "Float (single-precision)"))
  (`BlackboardComponent.SetValueAsBool` (`AIBlueprintHelperLibrary.GetBlackboard` null) "IsAttacking" (< (`self.GetDistanceTo` (`self.K2_GetPawn`) (`GameplayStatics.GetPlayerPawn` 0)) 125.0)))

(fn `UserConstructionScript`)