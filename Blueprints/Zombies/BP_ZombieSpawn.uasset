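; BP_ZombieSpawn is a spawn point that brings an existing zombie into play at its own location and rotation.
; CE_Spawn reactivates the passed-in zombie instead of creating one, moves it to the spawn transform and resets its mesh's relative transform.
; It then refills health to the given max, restores the capsule and mesh collision settings that death changes, plays its sound and re-enables its controller's tick.
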(event `CE_Spawn`
  (params (Zombie :type "/Game/Blueprints/Zombies/BP_Zombies Object Reference") (ZombieMaxHP :type "Float (double-precision)"))
  (bind _mesh (`Character.Mesh` Zombie))
  (bind _capsulecomponent (`Character.CapsuleComponent` Zombie))
  ;[1 1 1] Activate Zombie, Change Location/Rotation of Zombie and his Mesh Location/Rotation
  (`/Game/Blueprints/BP_FunctionLibrary.ActivateObject` Zombie)
  (`self.K2_SetActorLocationAndRotation` Zombie (`self.K2_GetActorLocation`) (`self.K2_GetActorRotation`) false false)
  (`SceneComponent.K2_SetRelativeLocationAndRotation` (`Character.Mesh` Zombie) (0.0 0.0 -90.0) (struct :`Yaw` -90.0) false false)
  ;[1 1 1] Change Health and Change Collisions settings because they change when a zombie dies
  (bind _output_get (set `/Game/Blueprints/Zombies/BP_Zombies.ZombieMaxHP` ZombieMaxHP Zombie))
  (set `/Game/Blueprints/Zombies/BP_Zombies.ZombieHP` _output_get Zombie)
  (`PrimitiveComponent.SetCollisionObjectType` _capsulecomponent "ECC_GameTraceChannel1")
  (`PrimitiveComponent.SetCollisionEnabled` _capsulecomponent "QueryAndPhysics")
  (`PrimitiveComponent.SetCollisionObjectType` _mesh "ECC_GameTraceChannel1")
  (`PrimitiveComponent.SetCollisionEnabled` _mesh "QueryAndPhysics")
  (`/Game/Blueprints/Zombies/BP_Zombies.CE_PlaySound` Zombie)
  ;[1 1 1] Enable Tick On Controller
  (`self.SetActorTickEnabled` (`/Game/Blueprints/Zombies/BP_Zombies.As BP Zombie Controller` Zombie) true))

(fn `UserConstructionScript`)