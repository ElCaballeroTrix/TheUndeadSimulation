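; Base game mode that runs round-based zombie waves with rising health, counts and fog.
; Timers activate pooled zombies at shuffled spawn points, adding MegaZombies on every fifth round.
; Once spawning ends, Tick checks that all zombies are hidden, then advances the round.
; Every fifth round pauses at a spawned checkpoint and saves round, money and score to the game instance; others start after a short delay.
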(event `CE_SpawnZombiesForPooling`
  ;[1 1 1] Spawn 30 for Object Pooling
  (for _ (range (+ (`self.ZombieAmountToPool`) 1))
    (bind _returnvalue (`|SpawnActorFromClass` "/Game/Blueprints/Zombies/BP_Zombies.BP_Zombies_C" (`KismetMathLibrary.MakeTransform` (0.0 0.0 1000.0) (`self.K2_GetActorRotation`)) "AdjustIfPossibleButAlwaysSpawn" "MultiplyWithRoot" null null))
    (set `self.ActorInPool` _returnvalue)
    (`/Game/Blueprints/BP_FunctionLibrary.ActivateObject` (`self.ActorInPool`) true)
    (`KismetArrayLibrary.Array_Add` (`self.ZombiePool`) (`self.ActorInPool`))))

(event `CE_IncreaseRound`
  ;[1 1 1] Increase Round
  (set `self.SpawnedAllZombies` false)
  (`/Engine/EditorBlueprintResources/StandardMacros.IncrementInt` (`self.RoundNumber`)
    (:`  `
      (set `self.MaxHealthOfZombies` (`KismetMathLibrary.Clamp` (select `bool` (< (`self.RoundNumber`) 10) :`false` (`KismetMathLibrary.FTrunc` (* (`self.MaxHealthOfZombies`) 1.1)) :`true` (+ (`self.MaxHealthOfZombies`) 100)) 0 10000))
      ;;[1 1 1] Start Round After 5 seconds unless round is a multiple of 5. In that case, there is a checkpoint
      (if (== (mod (`self.RoundNumber`) 5) 0)
        (bind _asbp_player (cast `/Game/Blueprints/Player/BP_Player` (`GameplayStatics.GetPlayerPawn` 0)))
        (bind _hud (`/Game/Blueprints/Player/BP_Player.HUD` _asbp_player))
        (`/Game/Blueprints/Interface/HUDS/WBP_HUD.CE_MessageText` _hud "Take a rest soldier and  \nhead back to the starting point \nto continue" "Visible" "/Game/Audio/Waves/S_Click.S_Click")
        (`KismetSystemLibrary.Delay` 4.0)
        (`/Game/Blueprints/Interface/HUDS/WBP_HUD.CE_MessageText` _hud "" "Hidden" null)
        (`self.SpawnCheckPoint`)
        ;;[1 1 1] Save Round Number, Money and Score When Checkpoint reached
        (bind _asbp_game_instance (cast `/Game/Blueprints/BP_GameInstance` (`GameplayStatics.GetGameInstance`)))
        (set `/Game/Blueprints/BP_GameInstance.Round` (`self.RoundNumber`) _asbp_game_instance)
        (bind _asbp_player_2 (cast `/Game/Blueprints/Player/BP_Player` (`GameplayStatics.GetPlayerPawn` 0)))
        (set `/Game/Blueprints/BP_GameInstance.Money` (`/Game/Blueprints/Player/BP_Player.Money` _asbp_player_2) _asbp_game_instance)
        (set `/Game/Blueprints/BP_GameInstance.Score` (`/Game/Blueprints/Player/BP_Player.Score` _asbp_player_2) _asbp_game_instance)
        (else
          (`KismetSystemLibrary.Delay` 5.0)
          (`self.CE_StartRound`))))))

(event `self.ReceiveTick`
  (params (DeltaSeconds :type "Float (single-precision)"))
  ;[1 1 1] Change Round when all zombies have spawned and are dead
  (if (`self.SpawnedAllZombies`)
    (bind _outactors (`GameplayStatics.GetAllActorsOfClass` "/Game/Blueprints/Zombies/BP_Zombies.BP_Zombies_C"))
    (for _array_element _outactors
      (if (`Actor.bHidden` _array_element)
        (set `self.AllZombiesDead` true)
        (else
          (set `self.AllZombiesDead` false)
          (break))))
    (if (`self.AllZombiesDead`)
      (`self.CE_IncreaseRound`)
      ;;[1 1 1] Fog is Increased
      (bind _returnvalue (`GameplayStatics.GetActorOfClass` "/Script/Engine.ExponentialHeightFog"))
      (bind _component (`ExponentialHeightFog.Component` _returnvalue))
      (`ExponentialHeightFogComponent.SetFogDensity` _component (`KismetMathLibrary.FClamp` (+ (`ExponentialHeightFogComponent.FogDensity` _component) 0.15) 0.0 10.0))
      (`GameplayStatics.PlaySound2D` "/Game/Audio/Waves/S_LevelComplete.S_LevelComplete" 1.0 1.0 0.0 null null))))

(event `CE_StartRound`
  ;[1 1 1] Start Round
  (`GameplayStatics.PlaySound2D` "/Game/Audio/Waves/S_RoundTransition.S_RoundTransition" 1.0 1.0 0.0 null null)
  (set `self.TotalZombiesInRound` (select `bool` (== (`self.RoundNumber`) 1) :`false` (`KismetMathLibrary.Round` (* (* (`self.RoundNumber`) 0.15) (`self.MaxZombies`))) :`true` 6))
  (bind _returnvalue (`KismetSystemLibrary.K2_SetTimerDelegate` (delegate `CE_SpawnZombie`) (`self.TimeBetweenSpawn`) true))
  ;;[1 1 1] If Round Number is Multiple of 5, Spawn MegaZombies as well
  (if (== (mod (`self.RoundNumber`) 5) 0)
    (bind _returnvalue_2 (`KismetSystemLibrary.K2_SetTimerDelegate` (delegate `CE_MegaZombieSpawn`) (* (`self.TimeBetweenSpawn`) 10.0) true))))

(event `CE_MegaZombieSpawn`
  (bind _megazombiesspawned (`self.MegaZombiesSpawned`))
  ;[1 1 1] Start Round
  ;;[1 1 1] If Round Number is Multiple of 5, Spawn MegaZombies as well
  (if (and (!= _megazombiesspawned 0) (== (mod _megazombiesspawned (`KismetMathLibrary.Clamp` (/ (`self.RoundNumber`) 5) 1 10)) 0))
    (`KismetSystemLibrary.K2_ClearAndInvalidateTimerHandle` (stale `CE_StartRound` _returnvalue_2))
    (set `self.MegaZombiesSpawned` 0)
    (else
      (bind _outactors (`GameplayStatics.GetAllActorsOfClass` "/Game/Blueprints/Zombies/BP_MegaZombieSpawn.BP_MegaZombieSpawn_C"))
      (`KismetArrayLibrary.Array_Shuffle` _outactors)
      (`/Game/Blueprints/Zombies/BP_MegaZombieSpawn.CE_MegaZombieSpawn` (`|GetArrayItem` _outactors) (`KismetMathLibrary.Conv_IntToDouble` (`self.MaxHealthOfZombies`)))
      (`/Engine/EditorBlueprintResources/StandardMacros.IncrementInt` (`self.MegaZombiesSpawned`)))))

(event `CE_SpawnZombie`
  ;[1 1 1] Start Round
  ;;[1 1 1] Spawn Zombie in a Spawner
  (if (< (`self.ZombiesSpawned`) (`self.TotalZombiesInRound`))
    (bind _outactors (`GameplayStatics.GetAllActorsOfClass` "/Game/Blueprints/Zombies/BP_ZombieSpawn.BP_ZombieSpawn_C"))
    (`KismetArrayLibrary.Array_Shuffle` _outactors)
    (bind _zombietoactivate (`self.GetAnInativeZombie`))
    (if (!= _zombietoactivate null)
      (`/Game/Blueprints/Zombies/BP_ZombieSpawn.CE_Spawn` (`|GetArrayItem` _outactors) _zombietoactivate (`KismetMathLibrary.Conv_IntToDouble` (`self.MaxHealthOfZombies`)))
      (`/Engine/EditorBlueprintResources/StandardMacros.IncrementInt` (`self.ZombiesSpawned`)))
    (else
      ;;[1 1 1] Detects when all zombies have spawned
      (`KismetSystemLibrary.K2_ClearAndInvalidateTimerHandle` (stale `CE_StartRound` _returnvalue))
      (set `self.ZombiesSpawned` 0)
      (set `self.SpawnedAllZombies` true))))

(fn `GetAnInativeZombie`
  (returns (ZombieToActivate :type "/Game/Blueprints/Zombies/BP_Zombies Object Reference"))
  (for _index (range (+ (`self.ZombieAmountToPool`) 1))
    (bind _output (`|GetArrayItem` (`self.ZombiePool`) _index))
    (if (not (`self.IsActorTickEnabled` _output))
      (return _output)))
  (return null))

(fn `UserConstructionScript`)