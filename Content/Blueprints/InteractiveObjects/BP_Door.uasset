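; BP_Door is a locked interactive door that the player opens with the interact input by spending a key.
; Overlap enables input and shows a HUD prompt; without a key, it plays a locked sound and message.
; Opening rotates DoorPivot through a timeline and enables the child BP_NavLink smart link, which is disabled at BeginPlay.
; Opened blocks further interaction, so the FlipFlop's closing branch is normally not reached.
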(event `self.ReceiveBeginPlay`
  ;[0.2001 1 0] BeginPlay
  (`EnhancedInputSubsystemInterface.AddMappingContext` (pcsubsystem `EnhancedInputLocalPlayerSubsystem` (`GameplayStatics.GetPlayerController` 0)) "/Game/ThirdPerson/Input/IMC_Default.IMC_Default" 0 (struct))
  (bind _asbp_nav_link (cast `/Game/Blueprints/Zombies/AI/BP_NavLink` (`ChildActorComponent.ChildActor` (`self.BP_NavLink`))))
  (`NavLinkProxy.SetSmartLinkEnabled` _asbp_nav_link false))

(event `self.ReceiveActorBeginOverlap`
  (params (OtherActor :type "Actor Object Reference"))
  ;[0 0 0] Overlaps
  (bind _ascharacter (cast `Character` OtherActor))
  (if (not (`self.Opened`))
    ;;[1 1 1] Access Player HUD
    (bind _asbp_player (cast `/Game/Blueprints/Player/BP_Player` _ascharacter))
    (set `self.As BP Player` _asbp_player)
    (bind _hud (`/Game/Blueprints/Player/BP_Player.HUD` _asbp_player))
    (set `self.HUD` _hud)
    (`/Game/Blueprints/Interface/HUDS/WBP_HUD.CE_MessageText` _hud "Press E to Open" "Visible" null)
    (`self.EnableInput` (`Pawn.GetLocalViewingPlayerController` _ascharacter))))

(event `self.ReceiveActorEndOverlap`
  (params (OtherActor :type "Actor Object Reference"))
  ;[0 0 0] Overlaps
  (bind _asbp_player (cast `/Game/Blueprints/Player/BP_Player` OtherActor))
  (`self.DisableInput` (`Pawn.GetLocalViewingPlayerController` _asbp_player))
  (`/Game/Blueprints/Interface/HUDS/WBP_HUD.CE_MessageText` (`self.HUD`) "\"\"" "Hidden" null))

(event `EnhancedInput|/Game/ThirdPerson/Input/Actions/IA_Interact`
  (params (ActionValue :type Boolean) (ElapsedSeconds :type "Float (double-precision)") (TriggeredSeconds :type "Float (double-precision)") (InputAction :type "InputAction Object Reference" :default "/Game/ThirdPerson/Input/Actions/IA_Interact.IA_Interact"))
  (bind _as_bp_player (`self.As BP Player`))
  (bind _numberofkeys (`/Game/Blueprints/Player/BP_Player.NumberOfKeys` _as_bp_player))
  ;[0 0 0] Open Door
  (:`Started`
    (if (== _numberofkeys 0)
      (if (not (`self.Opened`))
        ;;[1 1 1] Closed Door
        (`GameplayStatics.PlaySoundAtLocation` "/Game/Audio/Cues/S_DoorLockedCue.S_DoorLockedCue" (`self.K2_GetActorLocation`) (struct) 1.0 1.0 0.0 null null null null)
        (`/Game/Blueprints/Interface/HUDS/WBP_HUD.CE_MessageText` (`self.HUD`) "You need a Key" "Visible" "/Game/Audio/Cues/S_DoorLockedCue.S_DoorLockedCue"))
      (else
        ;;[1 1 1] If Player has a Key
        ;;;[1 1 1] If the door is already opened, it won't do anything
        (if (not (`self.Opened`))
          (bind _result (`/Engine/EditorBlueprintResources/StandardMacros.DecrementInt` _numberofkeys)
            (:`  `
              (set `/Game/Blueprints/Player/BP_Player.NumberOfKeys` _result _as_bp_player)
              ;;[1 1 1] Door Animation And Sound
              (`/Engine/EditorBlueprintResources/StandardMacros.DoOnce` false :!label _label
                (:`Completed`
                  (`/Engine/EditorBlueprintResources/StandardMacros.FlipFlop`
                    (:`A`
                      (`GameplayStatics.PlaySoundAtLocation` "/Game/Audio/Cues/S_DoorOpeningCue.S_DoorOpeningCue" (`self.K2_GetActorLocation`) (struct) 1.0 1.0 0.0 null null null null)
                      (bind (_direction _rotation) (`Timeline|Door Animation` :!label _label_2)
                        (:`Update`
                          (`SceneComponent.K2_SetRelativeRotation` (`self.DoorPivot`) (`KismetMathLibrary.MakeRotator` 0.0 0.0 _rotation) false false)
                          (set `self.Opened` true)
                          ;;[1 1 1] Smart Link
                          (bind _asbp_nav_link (cast `/Game/Blueprints/Zombies/AI/BP_NavLink` (`ChildActorComponent.ChildActor` (`self.BP_NavLink`))))
                          (`NavLinkProxy.SetSmartLinkEnabled` _asbp_nav_link true))
                        (:`Finished`
                          (goto _label :!via `Reset`))))
                    (:`B`
                      (`GameplayStatics.PlaySoundAtLocation` "/Game/Audio/Cues/S_DoorClosingCue.S_DoorClosingCue" (`self.K2_GetActorLocation`) (struct) 1.0 1.0 0.0 null null null null)
                      (goto _label_2 :!via `Reverse`))))))))))))

(fn `UserConstructionScript`
  (`SceneComponent.SetVisibility` (`self.Billboard`) (not (`self.Opened`)) false))