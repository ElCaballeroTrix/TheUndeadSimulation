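; BP_SniperAmmo_PickUp is an interactable ammo pickup that refills ammo for the weapon set in WeaponAffectedByAmmo.
; On CEInteract it searches the player's held weapons and acts only on a match.
; It sets that weapon's ammo in BP_GameInstance to its maximum, handling Pistol, Rifle, Shotgun and Sniper despite the sniper-specific name.
; It then triggers the player's reload and calls the parent interact.
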(event `/Game/Blueprints/InteractiveObjects/BP_InteractiveObject.CE_Interact`
  (bind _as_bp_game_instance (`self.As BP Game Instance`))
  (bind _as_bp_game_instance_2 (`self.As BP Game Instance`))
  (bind _as_bp_game_instance_3 (`self.As BP Game Instance`))
  (bind _as_bp_game_instance_4 (`self.As BP Game Instance`))
  (bind _asbp_player (cast `/Game/Blueprints/Player/BP_Player` (`GameplayStatics.GetPlayerPawn` 0)))
  (for _array_element (`/Game/Blueprints/Player/BP_Player.WeaponsHeld` _asbp_player)
    (if (`|EnumEquality` _array_element (`self.WeaponAffectedByAmmo`))
      (bind _asbp_game_instance (cast `/Game/Blueprints/BP_GameInstance` (`GameplayStatics.GetGameInstance`)))
      (set `self.As BP Game Instance` _asbp_game_instance)
      (switch `/Game/Blueprints/Enums/Enum_Weapons` (`self.WeaponAffectedByAmmo`)
        (:`NewEnumerator1`
          (set `/Game/Blueprints/BP_GameInstance.AmmoPistol` (`/Game/Blueprints/BP_GameInstance.MaxAmmoPistol` _as_bp_game_instance_3) _as_bp_game_instance_3))
        (:`NewEnumerator2`
          (set `/Game/Blueprints/BP_GameInstance.AmmoRifle` (`/Game/Blueprints/BP_GameInstance.MaxAmmoRifle` _as_bp_game_instance_4) _as_bp_game_instance_4))
        (:`NewEnumerator4`
          (set `/Game/Blueprints/BP_GameInstance.AmmoShotgun` (`/Game/Blueprints/BP_GameInstance.MaxAmmoShotgun` _as_bp_game_instance_2) _as_bp_game_instance_2))
        (:`NewEnumerator5`
          (set `/Game/Blueprints/BP_GameInstance.AmmoSniper` (`/Game/Blueprints/BP_GameInstance.MaxAmmoSniper` _as_bp_game_instance) _as_bp_game_instance)))
      (`/Game/Blueprints/Player/BP_Player.CE_ReloadWeapon` _asbp_player)
      (`parent.CE_Interact`)
      (break))))

(fn `UserConstructionScript`
  (`parent.UserConstructionScript`))