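; BP_SniperPickUp is a purchasable interactive sniper weapon pickup that the player buys with money.
; On interact it deducts the cost, then asks BP_Player to obtain the named weapon; success activates particles and runs the parent interact logic.
; Insufficient money shows a timed HUD error with sound.
; The cost is charged before the obtain check, and a failed obtain has no refund.
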(event `self.CE_Interact`
  (bind _as_bp_player (`self.As BP Player`))
  (bind _hud (`/Game/Blueprints/Player/BP_Player.HUD` (`self.As BP Player`)))
  (if (>= (`/Game/Blueprints/Player/BP_Player.Money` (`self.As BP Player`)) (`self.CostOfWeapon`))
    ;[1 1 1] Player Money Decreases
    (set `/Game/Blueprints/Player/BP_Player.Money` (- (`/Game/Blueprints/Player/BP_Player.Money` _as_bp_player) (`self.CostOfWeapon`)) _as_bp_player)
    (bind _asbp_player (cast `/Game/Blueprints/Player/BP_Player` (`GameplayStatics.GetPlayerPawn` 0)))
    (bind _weaponobtained (`/Game/Blueprints/Player/BP_Player.ObtainNewWeapon` _asbp_player (`self.WeaponName`)))
    (if _weaponobtained
      (`ActorComponent.Activate` (`self.Particles`) false)
      (`parent.CE_Interact`)
      (else
        (`KismetSystemLibrary.Delay` 2.0)
        (`/Game/Blueprints/Interface/HUDS/WBP_HUD.CE_MessageText` _hud "\"\"" "Hidden" null)))
    (else
      (`/Game/Blueprints/Interface/HUDS/WBP_HUD.CE_MessageText` _hud "You need more money" "Visible" "/Game/Audio/Cues/C_Error_Cue.C_Error_Cue")
      (`KismetSystemLibrary.Delay` 2.0)
      (`/Game/Blueprints/Interface/HUDS/WBP_HUD.CE_MessageText` _hud "\"\"" "Hidden" null))))

(fn `UserConstructionScript`
  (`parent.UserConstructionScript`))