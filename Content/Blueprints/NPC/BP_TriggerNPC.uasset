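; BP_TriggerNPC is an NPC trigger that sells keys to the player for money.
; Overlap shows a HUD offer and enables interact input, which is disabled when overlap ends.
; Interacting deducts the cost, raises the next price and spawns BP_Key at the Box, or briefly warns if funds are short.
; Purchases lock until the spawned key's OnDestroyed event re-enables them.
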(event `self.ReceiveActorBeginOverlap`
  (params (OtherActor :type "Actor Object Reference"))
  ;[1 1 1] NPC Overlap
  (if (`self.CanBuyKey`)
    (bind _asbp_player (cast `/Game/Blueprints/Player/BP_Player` OtherActor))
    (set `self.As BP Player` _asbp_player)
    (`self.EnableInput` (`GameplayStatics.GetPlayerController` 0))
    (`/Game/Blueprints/Interface/HUDS/WBP_HUD.CE_MessageText` (`/Game/Blueprints/Player/BP_Player.HUD` _asbp_player) (`KismetTextLibrary.Conv_StringToText` (`KismetStringLibrary.Concat_StrStr` "Would you like to buy a key for " (`KismetStringLibrary.Conv_IntToString` (`self.CostOfKey`)) "$")) "Visible" "/Game/Audio/Cues/C_HelloRobotCue.C_HelloRobotCue")))

(event `self.ReceiveActorEndOverlap`
  (params (OtherActor :type "Actor Object Reference"))
  ;[1 1 1] NPC Overlap
  (bind _asbp_player (cast `/Game/Blueprints/Player/BP_Player` OtherActor))
  (`self.DisableInput` (`GameplayStatics.GetPlayerController` 0))
  (`/Game/Blueprints/Interface/HUDS/WBP_HUD.CE_MessageText` (`/Game/Blueprints/Player/BP_Player.HUD` _asbp_player) "\"\"" "Hidden" null))

(event `EnhancedInput|/Game/ThirdPerson/Input/Actions/IA_Interact`
  (params (ActionValue :type Boolean) (ElapsedSeconds :type "Float (double-precision)") (TriggeredSeconds :type "Float (double-precision)") (InputAction :type "InputAction Object Reference" :default "/Game/ThirdPerson/Input/Actions/IA_Interact.IA_Interact"))
  (bind _as_bp_player (`self.As BP Player`))
  (bind _hud (`/Game/Blueprints/Player/BP_Player.HUD` (`self.As BP Player`)))
  ;[1 1 1] Spawn Key
  (:`Started`
    (if (>= (`/Game/Blueprints/Player/BP_Player.Money` (`self.As BP Player`)) (`self.CostOfKey`))
      ;;[1 1 1] Player Money Decreases
      (set `/Game/Blueprints/Player/BP_Player.Money` (- (`/Game/Blueprints/Player/BP_Player.Money` _as_bp_player) (`self.CostOfKey`)) _as_bp_player)
      ;;[1 1 1] Cost of Key Increases
      (set `self.CostOfKey` (+ (`self.CostOfKey`) 25))
      ;;[1 1 1] Spawn Key and forbids the player of buying another key until players obtains the key bought
      (bind _returnvalue (`|SpawnActorFromClass` "/Game/Blueprints/InteractiveObjects/PickUps/BP_Key.BP_Key_C" (`KismetMathLibrary.Conv_VectorToTransform` (`SceneComponent.K2_GetComponentLocation` (`self.Box`))) "Undefined" "MultiplyWithRoot" null null))
      (add `self.OnDestroyed` _returnvalue (delegate `CE_KeyObtained`))
      (set `self.CanBuyKey` false)
      (`self.DisableInput` (`GameplayStatics.GetPlayerController` 0))
      (else
        (`/Game/Blueprints/Interface/HUDS/WBP_HUD.CE_MessageText` _hud "You need more money" "Visible" "/Game/Audio/Cues/C_Error_Cue.C_Error_Cue")
        (`KismetSystemLibrary.Delay` 2.0)
        (`/Game/Blueprints/Interface/HUDS/WBP_HUD.CE_MessageText` _hud "\"\"" "Hidden" null)))))

(event `CE_KeyObtained` :!signature `self.OnDestroyed`
  (params (DestroyedActor :type "Actor Object Reference"))
  ;[1 1 1] Spawn Key
  ;;[1 1 1] Spawn Key and forbids the player of buying another key until players obtains the key bought
  (set `self.CanBuyKey` true))

(fn `UserConstructionScript`)