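; Bullet projectile that damages regular and Mega Zombies and gives hit feedback on impact.
; On a Box hit it plays an impact sound, adds a headshot sound for the "Spine2" bone, then casts the hit actor to each zombie type.
; Zombie hits apply damage, pass the result and headshot flag to the HUD and attach blood.
; Other hits spawn metal sparks, and every hit destroys the projectile.
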(event `self.Box.OnComponentHit`
  (params (HitComponent :type "PrimitiveComponent Object Reference") (OtherActor :type "Actor Object Reference") (OtherComp :type "PrimitiveComponent Object Reference") (NormalImpulse :type "Vector Structure") (Hit :type "HitResult Structure (by ref)"))
  (bind (_bblockinghit _binitialoverlap _time _distance _location _impactpoint _normal _impactnormal _physmat _hitactor _hitcomponent _hitbonename) (`GameplayStatics.BreakHitResult` Hit))
  (bind _returnvalue (== _hitbonename "Spine2"))
  ;[1 1 1] Bullet Logic
  (`GameplayStatics.PlaySoundAtLocation` (`self.ImpactSound`) _impactpoint (struct) 1.0 1.0 0.0 null null null null)
  ;;[1 0.902 0] If HeadShot, Play HeadShotSound
  (if _returnvalue
    (`GameplayStatics.PlaySoundAtLocation` "/Game/Audio/Cues/C_HeadShot_Cue.C_HeadShot_Cue" _impactpoint (struct) 1.0 1.0 0.0 null null null null))
  (bind _asbp_zombies (cast `/Game/Blueprints/Zombies/BP_Zombies` _hitactor)
    (:`then`
      ;;[1 1 1] Damage Zombies and Give Visual FeedBack
      (bind _dead (`/Game/Blueprints/Zombies/BP_Zombies.DamageZombie` _asbp_zombies (`self.ProjectileDamage`) _hitbonename _normal))
      (`/Game/Blueprints/Interface/HUDS/WBP_HUD.CE_HitEnemy` (`self.PlayerHUD`) _dead _returnvalue)
      (`GameplayStatics.SpawnEmitterAttached` "/Game/Realistic_Starter_VFX_Pack_Vol2/Particles/Blood/P_Blood_Splat_Cone.P_Blood_Splat_Cone" (`Character.Mesh` _asbp_zombies) "None" _impactpoint (`KismetMathLibrary.Conv_VectorToRotator` _impactpoint) (1.0 1.0 1.0) "KeepWorldPosition"))
    (:`CastFailed`
      ;;[1 1 1] Damage Mega Zombie and Give Visual FeedBack(Same Logic as with regular Zombie)
      (bind _asbp_mega_zombie (cast `/Game/Blueprints/Zombies/BP_MegaZombie` _hitactor)
        (:`then`
          (bind _dead_2 (`/Game/Blueprints/Zombies/BP_MegaZombie.DamageMegaZombie` _asbp_mega_zombie (`self.ProjectileDamage`) _hitbonename _normal))
          (`/Game/Blueprints/Interface/HUDS/WBP_HUD.CE_HitEnemy` (`self.PlayerHUD`) _dead_2 _returnvalue)
          (`GameplayStatics.SpawnEmitterAttached` "/Game/Realistic_Starter_VFX_Pack_Vol2/Particles/Blood/P_Blood_Splat_Cone.P_Blood_Splat_Cone" (`Character.Mesh` _asbp_mega_zombie) "None" _impactpoint (`KismetMathLibrary.Conv_VectorToRotator` _impactpoint)))
        (:`CastFailed`
          ;;[1 1 1] Spawn Different Emitter if Bullet didn't impact Enemy
          (`GameplayStatics.SpawnEmitterAtLocation` "/Game/MilitaryWeapSilver/FX/P_Impact_Metal_Medium_01.P_Impact_Metal_Medium_01" _impactpoint)))))
  (`self.K2_DestroyActor`))

(fn `UserConstructionScript`)