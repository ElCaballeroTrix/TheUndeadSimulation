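; AI controller for the mega zombie that runs its behavior tree and feeds it what perception senses of the player.
; Noise stimuli toggle PlayerFound false then true to force-restart investigation.
; Any other stimulus, treated as sight, sets PlayerSpotted to whether it was successfully sensed.
; Both kinds write the stimulus location to the InvestigateLocation blackboard key, and actors other than the player pawn are ignored.
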(event `self.ReceiveBeginPlay`
  ;[0.2901 1 0] Begin Play
  (`self.RunBehaviorTree` "/Game/Blueprints/Zombies/AI/BT_MegaZombieBehaviourTree.BT_MegaZombieBehaviourTree"))

(event `self.AIPerception.OnTargetPerceptionUpdated`
  (params (Actor :type "Actor Object Reference") (Stimulus :type "AIStimulus Structure"))
  (if (== Actor (`GameplayStatics.GetPlayerPawn` 0))
    (if (== Stimulus_Tag "Noise")
      ;[1 1 1] Force Restart Investigation
      (`BlackboardComponent.SetValueAsBool` (`self.Blackboard`) "PlayerFound" false)
      (`BlackboardComponent.SetValueAsBool` (`self.Blackboard`) "PlayerFound" true)
      (else
        ;[1 1 1] Sight
        (`BlackboardComponent.SetValueAsBool` (`self.Blackboard`) "PlayerSpotted" Stimulus_bSuccessfullySensed)))
    (`BlackboardComponent.SetValueAsVector` (`self.Blackboard`) "InvestigateLocation" Stimulus_StimulusLocation)))

(fn `UserConstructionScript`)