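; Zombie enemy character that damages the player through a hand collider, plays random groans and awards points when killed.
; DamageZombie doubles damage on Spine2 hits, treated as headshots, and triggers death at zero health, doubling points for headshot kills.
; Death ragdolls the body with an impulse, then either signals the Level1 gate (waypoint zombies) or rolls a rare item drop.
; The actor is then deactivated rather than destroyed, with its mesh reattached.
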(event `self.ReceiveBeginPlay`
  ;[0 1 0.0137] BeginPlay
  (bind _asbp_zombie_controller (cast `/Game/Blueprints/Zombies/AI/BP_ZombieController` (`AIBlueprintHelperLibrary.GetAIController` self)))
  (set `self.As BP Zombie Controller` _asbp_zombie_controller)
  (set `self.ZombieHP` (`self.ZombieMaxHP`))
  (`PrimitiveComponent.SetCollisionObjectType` (`self.CapsuleComponent`) "ECC_GameTraceChannel1")
  (`PrimitiveComponent.SetCollisionObjectType` (`self.Mesh`) "ECC_GameTraceChannel1"))

(event `CE_Die`
  (params (HeadShot :type Boolean) (Impulse :type "Vector Structure") (BoneName :type Name))
  ;[1 0 0.004057] Die
  (`PrimitiveComponent.SetCollisionObjectType` (`self.CapsuleComponent`) "ECC_Pawn")
  (`PrimitiveComponent.SetCollisionObjectType` (`self.Mesh`) "ECC_Pawn")
  ;;[1 1 1] Earn Points, Doble if HeadShot
  (bind _asbp_player (cast `/Game/Blueprints/Player/BP_Player` (`GameplayStatics.GetPlayerPawn` 0)))
  (if HeadShot
    (`/Game/Blueprints/BP_FunctionLibrary.AddPoints` (* (`self.PointsObtained`) 2) _asbp_player)
    (else
      (`/Game/Blueprints/BP_FunctionLibrary.AddPoints` (`self.PointsObtained`) _asbp_player)))
  (`self.SetActorTickEnabled` (`self.As BP Zombie Controller`) false)
  (`PrimitiveComponent.SetSimulatePhysics` (`self.Mesh`) true)
  (`PrimitiveComponent.SetCollisionEnabled` (`self.CapsuleComponent`) "NoCollision")
  (`PrimitiveComponent.SetCollisionResponseToChannel` (`self.Mesh`) "ECC_Visibility" "ECR_Ignore")
  (`PrimitiveComponent.AddImpulse` (`self.Mesh`) (* Impulse -10000.0) BoneName false)
  ;;[1 1 1] For Opening the Gate in Level1
  (if (`self.FollowsWaypoint`)
    (`self.Zombie1Died`)
    ;;[1 1 1] Disable Zombie
    (`KismetSystemLibrary.Delay` 3.0 :!label _label)
    (else
      ;;[1 1 1] Deactivate IsAttacking Blackboard Key
      (`BlackboardComponent.SetValueAsBool` (`AIBlueprintHelperLibrary.GetBlackboard` null) "IsAttacking" false)
      ;;[1 1 1] Probability of Spawning a Drop Once Dead
      (if (<= (`KismetMathLibrary.RandomFloat`) 0.05)
        (bind _returnvalue (`|SpawnActorFromClass` "/Game/Blueprints/InteractiveObjects/BP_Drop.BP_Drop_C" (`KismetMathLibrary.Conv_VectorToTransform` (`self.K2_GetActorLocation`)) "Undefined" "MultiplyWithRoot" null null))
        (`/Game/Blueprints/InteractiveObjects/BP_Drop.CE_DropItem` _returnvalue)
        (else
          (goto _label)))))
  (`/Game/Blueprints/BP_FunctionLibrary.ActivateObject` self true)
  (`PrimitiveComponent.SetSimulatePhysics` (`self.Mesh`) false)
  (`SceneComponent.K2_AttachToComponent` (`self.Mesh`) (`self.CapsuleComponent`) "None" "KeepRelative" "KeepRelative" "KeepRelative" true))

(event `self.HandCollider.OnComponentBeginOverlap`
  (params (OverlappedComponent :type "PrimitiveComponent Object Reference") (OtherActor :type "Actor Object Reference") (OtherComp :type "PrimitiveComponent Object Reference") (OtherBodyIndex :type Integer) (bFromSweep :type Boolean) (SweepResult :type "HitResult Structure (by ref)"))
  ;[1 1 1] Attack Player
  (if (`self.CanDamage`)
    (bind _asbp_player (cast `/Game/Blueprints/Player/BP_Player` OtherActor))
    (`/Game/Blueprints/BP_FunctionLibrary.TakeDamage` _asbp_player 10)
    (set `self.CanDamage` false)))

(event `CE_PlaySound`
  ;[1 1 1] Play a Zombie Sound at random time
  (if (`self.IsActorTickEnabled`) :!label _label_2
    (`KismetSystemLibrary.Delay` (`KismetMathLibrary.Conv_IntToDouble` (`KismetMathLibrary.RandomIntegerInRange` 10 20)))
    (if (`self.IsActorTickEnabled`)
      (`GameplayStatics.PlaySoundAtLocation` "/Game/Audio/Cues/C_ZombieSound_Cue.C_ZombieSound_Cue" (`self.K2_GetActorLocation`) (struct) 1.0 1.0 0.0 null null null null)
      (goto _label_2))))

(fn `DamageZombie`
  (params (Amount :type "Float (double-precision)") (BoneName :type Name) (ImpactPoint :type "Vector Structure"))
  (returns (Dead :type Boolean))
  (bind _returnvalue (== BoneName "Spine2"))
  (bind _output_get (set `self.ZombieHP` (`KismetMathLibrary.FClamp` (- (`self.ZombieHP`) (select `bool` _returnvalue :`false` Amount :`true` (* Amount 2.0))) 0.0 (`self.ZombieMaxHP`))))
  (bind _returnvalue_2 (== _output_get 0.0))
  (if _returnvalue_2
    (`self.CE_Die` _returnvalue ImpactPoint BoneName)
    (return _returnvalue_2)))

(fn `UserConstructionScript`)