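; Glass double-door actor whose two doors the player opens and closes individually with the E key.
; An InputBox overlap by FirstPersonCharacter enables input, while Box and Box1 set flags for which door is in range.
; E flip-flops that door's timeline forward or reverse, lerping its pivot's relative rotation to a target rotation.
; Door 1 takes priority when both flags are set.
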(event `self.Box.OnComponentBeginOverlap`
  (params (OverlappedComponent :type "PrimitiveComponent Object Reference") (OtherActor :type "Actor Object Reference") (OtherComp :type "PrimitiveComponent Object Reference") (OtherBodyIndex :type Integer) (bFromSweep :type Boolean) (SweepResult :type "HitResult Structure (by ref)"))
  (cast `/Game/MOUT_Civilian/Demo/FirstPersonBP/Blueprints/FirstPersonCharacter` OtherActor)
  (set `self.BoolDoor1` true))

(event `self.Box.OnComponentEndOverlap`
  (params (OverlappedComponent :type "PrimitiveComponent Object Reference") (OtherActor :type "Actor Object Reference") (OtherComp :type "PrimitiveComponent Object Reference") (OtherBodyIndex :type Integer))
  (cast `/Game/MOUT_Civilian/Demo/FirstPersonBP/Blueprints/FirstPersonCharacter` OtherActor)
  (set `self.BoolDoor1` false))

(event `Key|E`
  (params (Key :type "Key Structure"))
  (:`Pressed`
    (if (`self.BoolDoor1`)
      (`/Engine/EditorBlueprintResources/StandardMacros.FlipFlop`
        (:`A`
          (bind (_direction _alpha) (`Timeline|TL_OpenDoor1` :!label _label)
            (:`Update`
              (`SceneComponent.K2_SetRelativeRotation` (`self.Door1Pivot`) (`KismetMathLibrary.RLerp` (struct) (`self.Door 1 Rotation`) _alpha) false false))))
        (:`B`
          (goto _label :!via `Reverse`)))
      (elif (`self.BoolDoor2`)
        (`/Engine/EditorBlueprintResources/StandardMacros.FlipFlop`
          (:`A`
            (bind (_direction_2 _alpha_2) (`Timeline|TL_OpenDoor2` :!label _label_2)
              (:`Update`
                (`SceneComponent.K2_SetRelativeRotation` (`self.Door2Pivot`) (`KismetMathLibrary.RLerp` (struct) (`self.Door 2 Rotation`) _alpha_2) false false))))
          (:`B`
            (goto _label_2 :!via `Reverse`)))))))

(event `self.Box1.OnComponentBeginOverlap`
  (params (OverlappedComponent :type "PrimitiveComponent Object Reference") (OtherActor :type "Actor Object Reference") (OtherComp :type "PrimitiveComponent Object Reference") (OtherBodyIndex :type Integer) (bFromSweep :type Boolean) (SweepResult :type "HitResult Structure (by ref)"))
  (cast `/Game/MOUT_Civilian/Demo/FirstPersonBP/Blueprints/FirstPersonCharacter` OtherActor)
  (set `self.BoolDoor2` true))

(event `self.Box1.OnComponentEndOverlap`
  (params (OverlappedComponent :type "PrimitiveComponent Object Reference") (OtherActor :type "Actor Object Reference") (OtherComp :type "PrimitiveComponent Object Reference") (OtherBodyIndex :type Integer))
  (cast `/Game/MOUT_Civilian/Demo/FirstPersonBP/Blueprints/FirstPersonCharacter` OtherActor)
  (set `self.BoolDoor2` false))

(event `self.Input Box.OnComponentBeginOverlap`
  (params (OverlappedComponent :type "PrimitiveComponent Object Reference") (OtherActor :type "Actor Object Reference") (OtherComp :type "PrimitiveComponent Object Reference") (OtherBodyIndex :type Integer) (bFromSweep :type Boolean) (SweepResult :type "HitResult Structure (by ref)"))
  (cast `/Game/MOUT_Civilian/Demo/FirstPersonBP/Blueprints/FirstPersonCharacter` OtherActor)
  (`self.EnableInput` (`GameplayStatics.GetPlayerController` 0)))

(event `self.Input Box.OnComponentEndOverlap`
  (params (OverlappedComponent :type "PrimitiveComponent Object Reference") (OtherActor :type "Actor Object Reference") (OtherComp :type "PrimitiveComponent Object Reference") (OtherBodyIndex :type Integer))
  (cast `/Game/MOUT_Civilian/Demo/FirstPersonBP/Blueprints/FirstPersonCharacter` OtherActor)
  (`self.DisableInput` (`GameplayStatics.GetPlayerController` 0)))

(fn `UserConstructionScript`)